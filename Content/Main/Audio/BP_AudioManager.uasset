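; BP_AudioManager plays the game's ambient background audio: music, forest and wind.
; On BeginPlay it starts all three as non-positional 2D sounds.
; The music event re-triggers itself through a recursive four-minute Delay, while the forest and wind sounds are each fired once with no replay logic.
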(event Custom|PlayMusicAmbient
  (Audio|PlaySound2D (Variables|Default|GetAmbientMusic) 1.0 1.0 1.5 0 0)
  (Utilities|FlowControl|Delay 2.4e+02)
  (CallFunction|PlayMusicAmbient))

(event Custom|PlayForestAmbient
  (Audio|PlaySound2D (Variables|Default|GetAmbientForest) 1.0 1.0 0.0 0 0))

(event Custom|PlayWindAmbient
  (Audio|PlaySound2D (Variables|Default|GetAmbientWind) 1.0 1.0 0.0 0 0))

(event EventBeginPlay
  (CallFunction|PlayMusicAmbient)
  (CallFunction|PlayForestAmbient)
  (CallFunction|PlayWindAmbient))

(fn ConstructionScript)