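; BP_ItemObject is a world item actor that displays a configurable static mesh and reacts to interaction range.
; The construction script assigns ItemMesh to the mesh component.
; Entering or leaving interaction range toggles the mesh's custom depth rendering.
; Helper functions toggle physics simulation and overwrite the mesh's linear velocity.
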(event EventOnInteractionRangeEntered
  (Rendering|SetRenderCustomDepth (Variables|Debug|GetStaticMeshComponent) true))

(event EventOnInteractionRangeExit
  (Rendering|SetRenderCustomDepth (Variables|Debug|GetStaticMeshComponent) false))

(fn ConstructionScript
  (Components|StaticMesh|SetStaticMesh (Variables|Debug|GetStaticMeshComponent) (Variables|Default|GetItemMesh)))

(fn SetPhysicsEnabled
  (params (Enabled :type Boolean))
  (Physics|SetSimulatePhysics (Variables|Debug|GetStaticMeshComponent) Enabled))

(fn SetVelocity
  (params (Velocity :type Vector))
  (Class|PrimitiveComponent|SetAllPhysicsLinearVelocity (Variables|Debug|GetStaticMeshComponent) Velocity false))