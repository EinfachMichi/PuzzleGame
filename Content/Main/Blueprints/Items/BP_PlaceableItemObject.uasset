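; Base placeable item object that tracks how many times it can still be placed in the world.
; Place decrements PlaceCount, and IsPlaceable reports whether any placements remain.
; GetPlaceableActor returns the object itself, and the construction script only runs the parent's.
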(event EventPlace
  (Math|Integer|DecrementInt (Variables|Default|GetPlaceCount)))

(fn ConstructionScript
  (|CallParentFunction))

(fn GetPlaceableActor
  (return self))

(fn IsPlaceable
  (return (> (Variables|Default|GetPlaceCount) 0)))