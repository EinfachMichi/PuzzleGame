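; Game mode for a farming game that sequences NPC movement and relays task updates.
; On BeginPlay it takes the NPC list from the BP_NPCS actor and, after a short delay, triggers the first NPC's move.
; Each MoveNPC call moves the NPC at the Spawned index and increments it, quitting the game after a delay once the counter exceeds the list length.
; UpdateTaskEvent rebroadcasts task state through the OnTaskUpdate dispatcher.
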(event Custom|MoveNPC
  (Default|MOVE (Utilities|Array|Get(acopy) (Variables|Default|GetNPCs) (Variables|Default|GetSpawned)))
  (bind _result (Math|Integer|IncrementInt (Variables|Default|GetSpawned))
    (:%20%20
      (if (> _result (Utilities|Array|Length (Variables|Default|GetNPCs)))
        (Utilities|FlowControl|Delay 5.0)
        (Game|QuitGame 0 "Quit" false)))))

(event Custom|UpdateTaskEvent
  (params (Task :type S%20Task%20Structure) (CurrentTask :type S%20Task%20Structure) (Done :type Boolean))
  (Default|CallOnTaskUpdate Task CurrentTask Done))

(event EventBeginPlay
  (bind _returnvalue (Actor|GetActorOfClass "/Game/Main/Blueprints/BP_NPCS.BP_NPCS_C"))
  (Variables|Default|SetNPCs (Variables|/Game/Main/Blueprints/BP_NPCS.BP_NPCS_C|GetNPCS _returnvalue))
  (Utilities|FlowControl|Delay 1.0)
  (CallFunction|MoveNPC))

(fn ConstructionScript)