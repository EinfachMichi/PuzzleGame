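; BP_Shop is a shop in the farming system where a pawn browses items and buys one.
; On BeginPlay it binds click events on left arrow, right arrow and buy button components.
; The arrows call CycleThroughItems with opposite directions, and the buy button passes the clicking Pawn to BuyItem.
; The Blueprint only wires input, as the cycling and purchase logic are not defined in its graphs.
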(event Custom|RightButton
  (params (Pawn :type Pawn%20Object%20Reference))
  (Class|Shop|CycleThroughItems 1.0))

(event Custom|LeftButton
  (params (Pawn :type Pawn%20Object%20Reference))
  (Class|Shop|CycleThroughItems -1.0))

(event Custom|BuyButtonEvent
  (params (Pawn :type Pawn%20Object%20Reference))
  (Class|Shop|BuyItem Pawn))

(event EventBeginPlay
  (EventDispatchers|BindEventtoButtonClicked (Variables|Default|GetRightArrowButton) (EventDispatchers|CreateEvent :!event Custom|RightButton))
  (EventDispatchers|BindEventtoButtonClicked (Variables|Default|GetLeftArrowButton) (EventDispatchers|CreateEvent :!event Custom|LeftButton))
  (EventDispatchers|BindEventtoButtonClicked (Variables|Default|GetBuyButton) (EventDispatchers|CreateEvent :!event Custom|BuyButtonEvent)))

(fn ConstructionScript)