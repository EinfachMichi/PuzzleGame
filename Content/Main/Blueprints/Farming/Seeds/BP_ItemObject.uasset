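; BP_ItemObject is an interactable world item in the farming seeds folder that disappears when interacted with.
; The construction script applies the ItemMesh variable to its static mesh.
; Entering and leaving interaction range toggles the mesh's custom depth rendering.
; Interact waits one tick before destroying the actor and contains no other logic.
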(event EventInteract
  (Utilities|FlowControl|DelayUntilNextTick)
  (Actor|DestroyActor))

(event EventOnInteractionRangeEntered
  (Rendering|SetRenderCustomDepth (Variables|Default|GetStaticMesh) true))

(event EventOnInteractionRangeExit
  (Rendering|SetRenderCustomDepth (Variables|Default|GetStaticMesh) false))

(fn ConstructionScript
  (Components|StaticMesh|SetStaticMesh (Variables|Default|GetStaticMesh) (Variables|Default|GetItemMesh)))