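; NPC Blueprint that walks toward checkpoints, can be highlighted for interaction and consumes crops it touches.
; BeginPlay calls MoveToNextCheckpoint, which destroys the actor past the last checkpoint or runs AIMoveTo, only advancing the index on success without chaining another move.
; A custom-depth stencil outline shows while interactable; Interact disables and hides it.
; ItemEater overlaps destroy Crop actors with a Niagara effect at their location.
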(event OnComponentBeginOverlap(ItemEater)
  (params (OverlappedComponent :type Primitive%20Component%20Object%20Reference) (OtherActor :type Actor%20Object%20Reference) (OtherComp :type Primitive%20Component%20Object%20Reference) (OtherBodyIndex :type Integer) (bFromSweep :type Boolean) (SweepResult :type Hit%20Result%20Structure%20%28by%20ref%29))
  (bind _ascrop (Utilities|Casting|CastToCrop OtherActor))
  (Transformation|SetWorldLocation (Variables|Default|GetNiagara) (Transformation|GetActorLocation _ascrop) false true)
  (Components|Activation|Activate (Variables|Default|GetNiagara) false)
  (Actor|DestroyActor _ascrop))

(event Custom|MoveToNextCheckpoint
  (if (== (Variables|Default|GetCurrentCheckpoint) (Utilities|Array|Length (Variables|Default|GetCheckpoints)))
    (Actor|DestroyActor)
    (else
      (AI|AIMoveTo self (Utilities|Array|Get(acopy) (Variables|Default|GetCheckpoints) (Variables|Default|GetCurrentCheckpoint)) 0 5.0 false
        (:OnSuccess
          (bind _result (Math|Integer|IncrementInt (Variables|Default|GetCurrentCheckpoint))
            (:%20%20
              (Variables|Default|SetCurrentCheckpoint _result))))))))

(event Custom|ShowOutline
  (bind _mesh (Variables|Character|GetMesh))
  (if (Variables|Default|GetInteractable)
    (Rendering|SetRenderCustomDepth _mesh true)
    (Rendering|SetCustomDepthStencilValue _mesh 3)))

(event Custom|HideOutline
  (Rendering|SetRenderCustomDepth (Variables|Character|GetMesh) false))

(event Custom|Interact
  (Variables|Default|SetInteractable false)
  (CallFunction|HideOutline))

(event EventTick
  (params (DeltaSeconds :type Float%20%28single-precision%29))
  (if (Variables|Default|Get?Waiting)
    _))

(event EventBeginPlay
  (CallFunction|MovetoNextCheckpoint))

(fn ConstructionScript)